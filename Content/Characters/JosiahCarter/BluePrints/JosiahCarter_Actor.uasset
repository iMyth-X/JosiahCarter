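; Josiah Carter character actor whose animation follows a VR interactor's head position and whose facial states respond to player input.
; SetJosiahPosition multicasts from the server, copying the interactor camera's world location into the AnimBP's X, Y and Z; the equivalent Tick update is disconnected.
; Input events set talking, happy, angry, sad and shocked flags on the actor.
; The construction script attaches the feet collider to the mesh's hips socket.
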(event Custom|Assign%20Interactor%20Participant
  (params (Motion%20Controller%20Pawn :type New%20Motion%20Controller%20Pawn%20Object%20Reference))
  ;[1 1 1] Assign the VR Motion Control Pawn to local Interactor Pawn
  (Variables|Default|SetInteractorPawn Motion%20Controller%20Pawn))

(event Custom|MulticastSetJosiahPosition
  (params (Interactor :type New%20Motion%20Controller%20Pawn%20Object%20Reference))
  (bind _camera (Variables|/Game/VirtualRealityBP/Blueprints/NewMotionControllerPawn.NewMotionControllerPawn_C|GetCamera Interactor))
  (bind _returnvalue (Transformation|GetWorldLocation _camera))
  (bind (_x _y _z) (Math|Vector|BreakVector _returnvalue))
  ;[1 1 1] Get Position of the interactor from (Vive HMD/Camera) and broadcast to the server and all other clients
  (bind _asjosiah_carter_anim_bp (Utilities|Casting|CastToJosiahCarter_AnimBP (Components|SkeletalMesh|GetAnimInstance (Variables|Default|GetSkeletalMesh)))) ; Cast it to a Josiah Carter Actor instance
  (Utilities|IsValid _asjosiah_carter_anim_bp
    (:Is%20Valid
      (Variables|/Game/Characters/JosiahCarter/BluePrints/JosiahCarter_AnimBP.JosiahCarter_AnimBP_C|SetX _asjosiah_carter_anim_bp _x)
      (Variables|/Game/Characters/JosiahCarter/BluePrints/JosiahCarter_AnimBP.JosiahCarter_AnimBP_C|SetY _asjosiah_carter_anim_bp _y)
      (Variables|/Game/Characters/JosiahCarter/BluePrints/JosiahCarter_AnimBP.JosiahCarter_AnimBP_C|SetZ _asjosiah_carter_anim_bp _z))))

(event Custom|SetJosiahPosition
  (params (Interactor :type New%20Motion%20Controller%20Pawn%20Object%20Reference))
  ;[1 1 1] Trigger the Multicast Set Josiah Position Event (right Below)
  (Networking|SwitchHasAuthority
    (:Authority
      (CallFunction|MulticastSetJosiahPosition Interactor))))

(event EventBeginPlay)

(event Collision|EventActorBeginOverlap
  (params (OtherActor :type Actor%20Object%20Reference)))

(event EventTick
  (params (DeltaSeconds :type Float%20%28single-precision%29))
  ;[1 1 1] Get the position of the Interactor(Vive HMD/Camera) and send it to the AnimBP
  (Utilities|IsValid (Variables|Default|GetInteractorPawn) ; Interactor Pawn has been set up correctly?
    (:Is%20Valid
      (bind _asjosiah_carter_anim_bp (Utilities|Casting|CastToJosiahCarter_AnimBP (Components|SkeletalMesh|GetAnimInstance (Variables|Default|GetSkeletalMesh)))))))

(event Input|ActionEvents|InputActionInteractor_Happy
  (params (Key :type Key%20Structure :default "AnyKey"))
  ;[1 1 1] Face ANimation/States
  (:Pressed
    (Variables|Default|SetIsHappyBP true))
  (:Released
    (Variables|Default|SetIsHappyBP false)))

(event Input|ActionEvents|InputActionInteractor_Mad
  (params (Key :type Key%20Structure :default "AnyKey"))
  ;[1 1 1] Face ANimation/States
  (:Pressed
    (Variables|Default|SetIsAngryBP true))
  (:Released
    (Variables|Default|SetIsAngryBP false)))

(event Input|ActionEvents|InputActionInteractor_Sad
  (params (Key :type Key%20Structure :default "AnyKey"))
  ;[1 1 1] Face ANimation/States
  (:Pressed
    (Variables|Default|SetIsSadBP true))
  (:Released
    (Variables|Default|SetIsSadBP false)))

(event Input|ActionEvents|InputActionInteractor_Shock
  (params (Key :type Key%20Structure :default "AnyKey"))
  ;[1 1 1] Face ANimation/States
  (:Pressed
    (Variables|Default|SetIsShockedBP true))
  (:Released
    (Variables|Default|SetIsShockedBP false)))

(event Input|AxisEvents|InputAxisInteractorTalking
  (params (AxisValue :type Float%20%28single-precision%29))
  ;[1 1 1] Face ANimation/States
  (Variables|Default|SetIsTalkBP (Math|Conversions|ToBoolean(Integer) (Math|Float|Ceil AxisValue))))

(fn ConstructionScript
  ;[1 1 1] Remove the feet collider and attach to hips
  (Transformation|AttachComponentToComponent (Variables|Default|GetFeetCollider) (Variables|Default|GetSkeletalMesh) "HipsSocket" "KeepRelative" "KeepRelative" "KeepRelative" false))