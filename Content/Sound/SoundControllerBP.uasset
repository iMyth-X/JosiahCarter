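; Sound controller Blueprint that acts as a central wrapper for playing and stopping audio events, apparently FMOD.
; Play functions convert a sound identifier to an index into a Sounds array, then start the event at a location or attached to a component, with optional auto-play.
; Each returns the playing handle, and two stop functions halt either a component or an event instance.
; The event graph holds no logic.
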(event EventBeginPlay)

(event Collision|EventActorBeginOverlap
  (params (OtherActor :type Actor%20Object%20Reference)))

(event EventTick
  (params (DeltaSeconds :type Float%20%28single-precision%29)))

(fn ConstructionScript)

(fn PlaySoundatLocation
  (params (SoundToPlay :type SoundsEnum%20Enum) (PlayLocation :type Transform) (AutoPlay :type Boolean))
  (bind _returnvalue (Class|FMODBlueprintStatics|PlayEventatLocation (Utilities|Array|Get(acopy) (Variables|Default|GetSounds) (Math|Conversions|ToInteger(Byte) SoundToPlay)) PlayLocation AutoPlay))
  (return _returnvalue))

(fn PlaySoundAttached
  (params (Sound%20To%20Play :type SoundsEnum%20Enum) (Object%20to%20Attach%20To :type Scene%20Component%20Object%20Reference) (AutoPlay :type Boolean))
  (bind _returnvalue (Class|FMODBlueprintStatics|PlayEventAttached (Utilities|Array|Get(acopy) (Variables|Default|GetSounds) (Math|Conversions|ToInteger(Byte) Sound%20To%20Play)) Object%20to%20Attach%20To "None" "0, 0, 0" "KeepRelativeOffset" false AutoPlay))
  (return _returnvalue))

(fn StopSoundReference
  (params (Component%20to%20stop :type FMOD%20Audio%20Component%20Object%20Reference))
  (Class|FMODAudioComponent|Stop Component%20to%20stop))

(fn StopEvent
  (params (Event%20to%20stop :type FMOD%20Event%20Instance%20Structure))
  (Class|FMODBlueprintStatics|EventInstanceStop Event%20to%20stop))