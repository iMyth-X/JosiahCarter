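; VR game instance Blueprint that stores the GameManager reference and broadcasts when it is received.
; Its host, join and control-panel events are empty stubs.
; Disconnected, never-run graphs hold LAN session hosting and joining, Audio and Director panel creation, and actor-type setup for Sound Client and Director roles.
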(event Custom|InstanceHost
  (params (PlayerController :type Player%20Controller%20Object%20Reference)))

(event Custom|DisplayAudioControlPanel)

(event Custom|DisplayDirectorControlPanel)

(event Custom|InstanceJoin
  (params (PlayerController :type Player%20Controller%20Object%20Reference)))

(fn SetGameManager
  (params (GameManager :type BP%20Game%20Manager%20Object%20Reference%20%28by%20ref%29))
  (bind _output_get (Variables|Default|SetGameManagerRef GameManager))
  (Default|CallOnGameManagerReceived _output_get))

(fn GetGameManager
  (return (Variables|Default|GetGameManagerRef)))