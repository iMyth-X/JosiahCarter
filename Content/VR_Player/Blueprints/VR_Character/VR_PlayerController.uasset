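; VR player controller that lets a user host or join a networked session and take control of a motion controller pawn.
; H and J key releases each fire once, passing the controller to the VR game instance's host or join function.
; BeginPlay derives the actor type from the interactor setting, falling back to participant when none is set.
; A custom event spawns the motion controller pawn at the controller's location and possesses it.
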(event Custom|Host
  ;[1 1 1] ACtion to Take if process is Host
  (bind _asmy_vrgame_instance_bp (Utilities|Casting|CastToMyVRGameInstanceBP (Game|GetGameInstance)))
  (Default|InstanceHost _asmy_vrgame_instance_bp self))

(event Custom|Join
  ;[1 1 1] ACtion to take if Process is Join
  (bind _asmy_vrgame_instance_bp (Utilities|Casting|CastToMyVRGameInstanceBP (Game|GetGameInstance)))
  (Default|InstanceJoin _asmy_vrgame_instance_bp self))

(event Custom|CreatePawnToPossess
  ;[1 1 1] Spawn a new Motion controller pawn
  (bind _returnvalue (Game|SpawnActorfromClass "/Game/VirtualRealityBP/Blueprints/NewMotionControllerPawn.NewMotionControllerPawn_C" (Math|Conversions|ToTransform(Vector) (Transformation|GetWorldLocation (Variables|Default|GetTransformComponent))) "Undefined" 0 0))
  (Pawn|Possess _returnvalue))

(event EventBeginPlay
  ;[1 1 1] Set the Actor type to whatever but if there is no actor type then set to participant by default
  (bind _output_get (Variables|Default|SetActorType (Utilities|Enum|ByteToEnumNetworkComponentEnum (stale _output_get))))
  (if (Utilities|Enum|Equal(Enum) _output_get "NewEnumerator4")
    (Variables|Default|SetActorType "NewEnumerator0")))

(event Input|KeyboardEvents|H
  (params (Key :type Key%20Structure :default "AnyKey"))
  ;[1 1 1] Press 'h' to set process as Host
  (:Released
    (Utilities|FlowControl|DoOnce false
      (:Completed
        (CallFunction|Host)))))

(event Input|KeyboardEvents|J
  (params (Key :type Key%20Structure :default "AnyKey"))
  ;[1 1 1] Press 'j' top joint the existing experience
  (:Released
    (Utilities|FlowControl|DoOnce false
      (:Completed
        (CallFunction|Join)))))

(fn ConstructionScript)