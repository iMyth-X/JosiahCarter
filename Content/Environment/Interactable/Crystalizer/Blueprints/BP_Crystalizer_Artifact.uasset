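; BP_Crystalizer_Artifact is an interactable Crystalizer artifact that triggers a world transition in a VR game.
; When interaction begins, it gets the game manager through MyVRGameInstanceBP, plays the crystallizer activation sound, then calls StartWorldTransition.
; If the game instance cast fails, neither the sound nor the transition runs.
; GetArtifactColor supplies a fixed cyan as the artifact's color.
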(event EventBeginPlay
  (|CallParentFunction))

(event Collision|EventActorBeginOverlap
  (params (OtherActor :type Actor%20Object%20Reference)))

(event EventTick
  (params (DeltaSeconds :type Float%20%28single-precision%29)))

(event EventOnInteractionBegin
  (params (SilverKey :type BP%20Silver%20Key%20Object%20Reference))
  (bind _asmy_vrgame_instance_bp (Utilities|Casting|CastToMyVRGameInstanceBP (Game|GetGameInstance)))
  (Default|PlayCrystallizerActivationSound (Default|GetGameManager _asmy_vrgame_instance_bp))
  (CallFunction|StartWorldTransition))

(fn ConstructionScript
  (|CallParentFunction))

(fn GetArtifactColor
  (return "(R=0.000000,G=1.000000,B=1.000000,A=1.000000)"))