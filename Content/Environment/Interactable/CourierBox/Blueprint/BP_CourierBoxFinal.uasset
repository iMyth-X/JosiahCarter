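; Courier box actor whose lid swings open when OpenBox is called.
; OpenBox runs once, playing a timeline at a rate set by OpeningSpeed that rolls LidAnchor in world space.
; Tick can also pitch BoxLid from a Vive controller's height while Opening is set, but the grab logic that sets it is disconnected.
; Openable, Pickup and Drop events are empty, with their former attach and physics logic left unwired.
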(event Custom|OpenBox
  (params (OpeningSpeed :type Float%20%28single-precision%29))
  (bind _lidanchor (Variables|Default|GetLidAnchor))
  (bind _returnvalue (Transformation|GetWorldRotation _lidanchor))
  (Utilities|FlowControl|DoOnce false
    (:Completed
      (Components|Timeline|SetPlayRate (Variables|Default|GetOpenBoxTimeline) (/ 1.0 OpeningSpeed))
      (bind _lidangle (Timeline|OpenBoxTimeline Play)
        (:Update
          (Transformation|SetWorldRotation _lidanchor (Math|Rotator|MakeRotator _lidangle (.pitch _returnvalue) (.yaw _returnvalue)) false false))))))

(event EventBeginPlay)

(event EventPickup
  (params (AttachTo :type Scene%20Component%20Object%20Reference))
  ;[1 1 1] Pickup Item
)

(event EventDrop
  ;[1 1 1] Drop Items
)

(event EventTick
  (params (DeltaSeconds :type Float%20%28single-precision%29))
  (bind _boxbody (Variables|Default|GetBoxBody))
  (bind _vivecontrollerref (Variables|Default|GetViveControllerRef))
  (bind _vcontrollerpos (Variables|OldCode|GetVControllerPos))
  (bind _boxlid (Variables|Default|GetBoxLid))
  (bind _returnvalue (Transformation|GetWorldLocation _boxbody))
  (bind _z (Math|Vector|BreakVector _vcontrollerpos))
  (bind _returnvalue_2 (Transformation|GetWorldLocation _vivecontrollerref))
  (bind _relativerotation (Variables|/Script/Engine.SceneComponent|GetRelativeRotation _boxlid))
  (bind _returnvalue_3 (- (.z _returnvalue_2) (.z _returnvalue)))
  (bind _returnvalue_4 (- _returnvalue_3 _z))
  (bind _returnvalue_5 (* _returnvalue_4 -1.1))
  ;[1 1 1] Event Tick
  (if (Variables|OldCode|GetOpening)
    (Utilities|IsValid _vivecontrollerref
      (:Is%20Valid
        (if (> _returnvalue_4 0.0)
          (if (<= _returnvalue_4 9e+01)
            (Variables|OldCode|SetRotationReference _returnvalue_5)
            (Transformation|SetRelativeRotation (Variables|Default|GetBoxLid) (Math|Rotator|MakeRotator (.roll _relativerotation) _returnvalue_5 (.yaw _relativerotation)) false false))))
      (:Is%20Not%20Valid
        (Variables|OldCode|SetOpening false)))))

(event EventOpenable
  ;[1 1 1] Opening event
)

(fn ConstructionScript)