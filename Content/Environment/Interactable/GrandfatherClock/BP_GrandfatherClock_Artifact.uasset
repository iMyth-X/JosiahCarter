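; Interactable grandfather clock artifact for a VR game that, on its first interaction, rings through the Game Manager and starts a world transition.
; The construction script derives each hand's rotation rate from seconds per revolution and poses the hands at the initial time.
; Tick accumulates time scaled by an adjustable SpeedOfTime, then sets hand roll from that total.
; An incremental UpdateClockTime variant exists but is not called here.
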(event Collision|EventActorBeginOverlap
  (params (OtherActor :type Actor%20Object%20Reference)))

(event EventTick
  (params (DeltaSeconds :type Float%20%28single-precision%29))
  (CallFunction|ClockTick DeltaSeconds))

(event EventOnInteractionBegin
  (params (SilverKey :type BP%20Silver%20Key%20Object%20Reference))
  (Utilities|FlowControl|DoOnce false
    (:Completed
      (bind _asmy_vrgame_instance_bp (Utilities|Casting|CastToMyVRGameInstanceBP (Game|GetGameInstance)))
      (Default|PlayClockRingSound (Default|GetGameManager _asmy_vrgame_instance_bp))
      (CallFunction|StartWorldTransition))))

(event EventOnInteractionEnd
  (params (SilverKey :type BP%20Silver%20Key%20Object%20Reference)))

(event EventOnInteractionHit
  (params (SilverKey :type BP%20Silver%20Key%20Object%20Reference)))

(event EventBeginPlay
  (|CallParentFunction))

(fn ConstructionScript
  (Utilities|FlowControl|Sequence
    (:then_0
      (|CallParentFunction))
    (:then_1
      (Variables|Default|SetHandList (Utilities|Array|MakeArray (Variables|Default|GetHourHandAnchor) (Variables|Default|GetMinuteHandAnchor)))
      (for _array_element (Variables|Default|GetHandSecondsPerRotationList)
        (Utilities|Array|Add (Variables|Default|GetHandRotateSpeedList) (/ -3.6e+02 (Math|Conversions|ToFloat(Integer) _array_element)))))
    (:then_2
      (bind _output_get (Variables|Default|SetTotalTime (+ (* (Variables|Default|GetInitialHour) 3.6e+03) (* (Variables|Default|GetInitialMinute) 6e+01))))
      (CallFunction|SetClockTime _output_get))))

(fn GetArtifactColor
  (return "(R=1.000000,G=0.171748,B=0.000000,A=1.000000)"))

(fn ClockTick
  (params (DeltaTime :type Float%20%28single-precision%29))
  (bind _output_get (LocalVariables|SetNewDeltaTime (* DeltaTime (Variables|Default|GetSpeedOfTime))))
  (bind _output_get_2 (Variables|Default|SetTotalTime (+ _output_get (Variables|Default|GetTotalTime))))
  (CallFunction|SetClockTime _output_get_2))

(fn SetClockTime
  (params (TimeSinceStart :type Float%20%28single-precision%29))
  (for _index (range 0 (- (Variables|Default|GetNumberOfHands) 1))
    (Transformation|SetRelativeRotation (Utilities|Array|Get(acopy) (Variables|Default|GetHandList) _index) (Math|Rotator|MakeRotator (* (Utilities|Array|Get(acopy) (Variables|Default|GetHandRotateSpeedList) _index) TimeSinceStart) (.Pitch (Math|Rotator|BreakRotator (Variables|/Script/Engine.SceneComponent|GetRelativeRotation (Utilities|Array|Get(acopy) (Variables|Default|GetHandList) _index)))) (.Yaw (Math|Rotator|BreakRotator (Variables|/Script/Engine.SceneComponent|GetRelativeRotation (Utilities|Array|Get(acopy) (Variables|Default|GetHandList) _index))))) false false)))

(fn UpdateClockTime
  (params (DeltaTime :type Float%20%28single-precision%29))
  (for _index (range 0 (- (Variables|Default|GetNumberOfHands) 1))
    (Transformation|SetRelativeRotation (Utilities|Array|Get(acopy) (Variables|Default|GetHandList) _index) (Math|Rotator|MakeRotator (+ (.Roll (Math|Rotator|BreakRotator (Variables|/Script/Engine.SceneComponent|GetRelativeRotation (Utilities|Array|Get(acopy) (Variables|Default|GetHandList) _index)))) (* (Utilities|Array|Get(acopy) (Variables|Default|GetHandRotateSpeedList) _index) DeltaTime)) (.Pitch (Math|Rotator|BreakRotator (Variables|/Script/Engine.SceneComponent|GetRelativeRotation (Utilities|Array|Get(acopy) (Variables|Default|GetHandList) _index)))) (.Yaw (Math|Rotator|BreakRotator (Variables|/Script/Engine.SceneComponent|GetRelativeRotation (Utilities|Array|Get(acopy) (Variables|Default|GetHandList) _index))))) false false)))

(fn SetClockSpeed
  (params (Speed :type Float%20%28single-precision%29))
  (Variables|Default|SetSpeedOfTime Speed))