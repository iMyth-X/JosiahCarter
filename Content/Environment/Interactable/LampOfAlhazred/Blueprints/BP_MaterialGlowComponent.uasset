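; Component that gives its owner's static meshes dynamic materials built from texture sets, with shared emissive glow control, stored under the Lamp of Alhazred interactable.
; Construction counts material slots, auto-fills an empty mesh-to-texture mapping, then builds a mesh list parallel to the texture array.
; Each slot gets an opaque or transparent dynamic instance, collected for the emissive color and intensity setters.
; BeginPlay clears the texture and mapping arrays.
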(event EventBeginPlay
  ;[1 1 0] NEW!
  (Utilities|Array|Clear (Variables|Parameters|GetElementTexture))
  (Utilities|Array|Clear (Variables|Parameters|GetMeshNameToTextureMapping)))

(event EventConstructionScript
  (bind _meshinfolist (Variables|Information|GetMeshInfoList))
  ;[1 1 0] NEW!
  (Utilities|FlowControl|Sequence
    (:then_0
      ;;[1 1 1] Get Number of Static Meshes
      (Variables|Information|SetNumberOfMaterials 0)
      (for _array_element (Actor|GetComponentsByClass (Components|GetOwner) "/Script/Engine.StaticMeshComponent")
        (Variables|Information|SetNumberOfMaterials (+ (Variables|Information|GetNumberOfMaterials) (Rendering|Material|GetNumMaterials _array_element)))))
    (:then_1
      ;;[1 1 1] Set the number of Element Textures
      (Utilities|Array|Resize (Variables|Parameters|GetElementTexture) (Variables|Information|GetNumberOfMaterials))
      ;;[1 1 1] Auto-Fill the Mesh to Texture Mapping if empty
      (if (== (Utilities|Array|Length (Variables|Parameters|GetMeshNameToTextureMapping)) 0)
        (bind (_staticmesh _materialindex _overallindex) (Utilities|ForEachMaterial (Components|GetOwner))
          (:LoopBody
            (Utilities|Array|Add (Variables|Parameters|GetMeshNameToTextureMapping) (Utilities|Struct|MakeMatTexPair (Utilities|GetObjectName _staticmesh) _materialindex _overallindex))))))
    (:then_2
      ;;[1 1 1] Update Mesh Info List based on Mesh to Texture Mapping (and make it to be parallel to Element Texture)
      (Utilities|Array|Clear _meshinfolist)
      (Utilities|Array|Resize _meshinfolist (Variables|Information|GetNumberOfMaterials))
      (bind (_staticmesh_2 _materialindex_2) (Utilities|ForEachMaterial (Components|GetOwner))
        (:LoopBody
          (bind _array_element_2 (Utilities|Array|ForEachLoopwithBreak (Variables|Parameters|GetMeshNameToTextureMapping) :!label _label)
            (:LoopBody
              (if (== _materialindex_2 (.MaterialIndex (Utilities|Struct|BreakMatTexPair _array_element_2)))
                (if (Utilities|Enum|Equal(Enum) (Utilities|GetObjectName _staticmesh_2) (.MeshName (Utilities|Struct|BreakMatTexPair _array_element_2)))
                  (Utilities|Array|SetArrayElem (Variables|Information|GetMeshInfoList) (Math|Integer|Clamp(Integer) (.ElementTextureIndex (Utilities|Struct|BreakMatTexPair _array_element_2)) 0 (Utilities|Array|LastIndex (Variables|Parameters|GetElementTexture))) (Utilities|Struct|MakeMeshInfo _staticmesh_2 (.MaterialIndex (Utilities|Struct|BreakMatTexPair _array_element_2))))
                  (goto _label Break))))))))
    (:then_3
      ;;[1 1 1] Set-Up the Dynamic Material Lists
      (CallFunction|ClearMaterialLists)
      (for (_array_element_3 _array_index) (Variables|Information|GetMeshInfoList)
        (bind _currentmaterial (CallFunction|InitializeMaterialListElementsfromTextureBuffer (Utilities|Array|Get(acopy) (Variables|Parameters|GetElementTexture) (Math|Integer|Clamp(Integer) _array_index 0 (Utilities|Array|LastIndex (Variables|Parameters|GetElementTexture))))))
        (Rendering|Material|SetMaterial (.mesh _array_element_3) (.materialindex _array_element_3) _currentmaterial)))))

(fn CreateMaterialDynamic
  (params (Parent :type Material%20Interface%20Object%20Reference) (Textures :type Texture%20Buffer%20Structure%20%28by%20ref%29))
  (bind _returnvalue (Rendering|Material|CreateDynamicMaterialInstance Parent :!class /Script/Engine.KismetMaterialLibrary))
  (Rendering|Material|SetTextureParameterValue _returnvalue "Base" (.base Textures))
  (Rendering|Material|SetTextureParameterValue _returnvalue "MetRoughAO" (.metroughao Textures))
  (Rendering|Material|SetTextureParameterValue _returnvalue "Normal" (.normal Textures))
  (Rendering|Material|SetTextureParameterValue _returnvalue "Emissive" (.emissive Textures))
  (Rendering|Material|SetTextureParameterValue _returnvalue "Opacity" (.opacity Textures))
  (Rendering|Material|SetScalarParameterValue _returnvalue "Tiling" (Math|Conversions|ToFloat(Integer) (.tiling Textures)) :!class /Script/Engine.MaterialInstanceDynamic)
  (return _returnvalue))

(fn SetEmissiveColor
  (params (EmissiveColor :type Linear%20Color%20Structure))
  (for _array_element (Variables|Default|GetNormalMaterialList)
    (Rendering|Material|SetVectorParameterValue _array_element "EmissiveColor" EmissiveColor :!class /Script/Engine.MaterialInstanceDynamic)))

(fn SetEmissiveIntensity
  (params (Intensity :type Float%20%28single-precision%29))
  (for _array_element (Variables|Default|GetNormalMaterialList)
    (Rendering|Material|SetScalarParameterValue _array_element "EmissiveIntensity" Intensity :!class /Script/Engine.MaterialInstanceDynamic)))

(fn CreateElementTexture
  (params (Size :type Integer))
  (bind _localarray (LocalVariables|GetLocalArray))
  (Utilities|Array|Resize _localarray Size)
  (return _localarray))

(fn InitializeMaterialListElementsfromTextureBuffer
  (params (TextureBuffer :type Texture%20Buffer%20Structure%20%28by%20ref%29))
  (if (.bIsTransparent (Utilities|Struct|BreakTextureBuffer TextureBuffer))
    (bind _dynamicmaterial (CallFunction|CreateMaterialDynamic "/Game/Environment/Interactable/LampOfAlhazred/Materials/M_TransparentMaterial.M_TransparentMaterial" TextureBuffer))
    (LocalVariables|SetNormalMaterial _dynamicmaterial)
    (else
      (bind _dynamicmaterial_2 (CallFunction|CreateMaterialDynamic "/Game/Environment/Interactable/LampOfAlhazred/Materials/M_NormalMaterial.M_NormalMaterial" TextureBuffer))
      (LocalVariables|SetNormalMaterial _dynamicmaterial_2)))
  (Utilities|Array|Add (Variables|Default|GetNormalMaterialList) (LocalVariables|GetNormalMaterial))
  (return (LocalVariables|GetNormalMaterial)))

(fn SetDynamicMaterials)

(fn ClearMaterialLists
  (Utilities|Array|Clear (Variables|Default|GetNormalMaterialList))
  (return))