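; Lamp of Alhazred transition sphere: a growing and shrinking light volume that drives a world transition on nearby objects.
; Overlaps register BP_MaterialTransformComponents with the parent's BP_TransitionManager, and the sphere pushes its position and radius to them by light index.
; Start/Stop play or reverse a timeline scaling the radius, triggering enter/exit on toggle-list actors.
; Construction pre-gathers affected static objects, hidden after expansion and shown again on reversal.
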(event OnComponentBeginOverlap(SphereCollider)
  (params (OverlappedComponent :type Primitive%20Component%20Object%20Reference) (OtherActor :type Actor%20Object%20Reference) (OtherComp :type Primitive%20Component%20Object%20Reference) (OtherBodyIndex :type Integer) (bFromSweep :type Boolean) (SweepResult :type Hit%20Result%20Structure%20%28by%20ref%29))
  (CallFunction|OnLightBeginOverlap OtherActor OtherComp))

(event OnComponentEndOverlap(SphereCollider)
  (params (OverlappedComponent :type Primitive%20Component%20Object%20Reference) (OtherActor :type Actor%20Object%20Reference) (OtherComp :type Primitive%20Component%20Object%20Reference) (OtherBodyIndex :type Integer))
  (CallFunction|OnLightEndOverlap OtherActor OtherComp))

(event Custom|OnLightBeginOverlap
  (params (OtherActor :type Actor%20Object%20Reference) (OtherComp :type Primitive%20Component%20Object%20Reference))
  (bind _returnvalue (Actor|GetComponentbyClass OtherActor "/Game/Environment/Interactable/LampOfAlhazred/Blueprints/BP_MaterialTransformComponent.BP_MaterialTransformComponent_C"))
  (Utilities|IsValid _returnvalue
    (:Is%20Valid
      (Utilities|Array|AddUnique (Variables|Default|GetLitObjectList) _returnvalue)
      (Default|AddLitObject (Variables|Default|GetTransitionManagerRef) self _returnvalue))))

(event Custom|StartWorldTransition
  (Utilities|FlowControl|Sequence
    (:then_0
      (Utilities|FlowControl|DoOnce false
        (:Completed
          (Utilities|FlowControl|Sequence
            (:then_0
              ;[1 1 1] World Transition Timeline
              (bind (_direction _transitionspeed) (Timeline|TransitionTimeline Play)
                (:Update
                  (CallFunction|UpdateProperties (* (Variables|Default|GetInitialLightRadius) _transitionspeed))
                  (Development|PrintString (Utilities|String|ToString(Float) (* (Variables|Default|GetInitialLightRadius) _transitionspeed)) true false "(R=1.000000,G=0.000000,B=0.909153,A=1.000000)" 0.03))
                (:Finished
                  ;[1 1 1] End of Transition, Hide Actors that are no longer visible
                  (switch Utilities|FlowControl|Switch|SwitchonETimelineDirection _direction
                    (:Forward
                      (Rendering|SetActorHiddenInGame (Variables|Information|GetAffectedObjects) true))
                    (:Backward
                      ;[1 1 1] Beginning of Transition, Appear/Disappear Actors
                      (for _array_element (Variables|Parameters|GetTransitionToggleList)
                        (Default|ExitTransition _array_element)))))))
            (:then_1
              (Utilities|FlowControl|Delay (Variables|Parameters|GetBeginTimeOffset))
              (for _array_element_2 (Variables|Parameters|GetTransitionToggleList)
                (Default|EnterTransition _array_element_2)))))))
    (:then_1
      (Utilities|FlowControl|DoOnce true) ; enters at Reset
    )))

(event Custom|StopWorldTransition
  (Utilities|FlowControl|Sequence
    (:then_0
      (Utilities|FlowControl|DoOnce true
        (:Completed
          (Utilities|FlowControl|Sequence
            (:then_0
              ;[1 1 1] World Transition Timeline
              (bind (_direction _transitionspeed) (Timeline|TransitionTimeline Reverse)
                (:Update
                  (CallFunction|UpdateProperties (* (Variables|Default|GetInitialLightRadius) _transitionspeed))
                  (Development|PrintString (Utilities|String|ToString(Float) (* (Variables|Default|GetInitialLightRadius) _transitionspeed)) true false "(R=1.000000,G=0.000000,B=0.909153,A=1.000000)" 0.03))
                (:Finished
                  ;[1 1 1] End of Transition, Hide Actors that are no longer visible
                  (switch Utilities|FlowControl|Switch|SwitchonETimelineDirection _direction
                    (:Forward
                      (Rendering|SetActorHiddenInGame (Variables|Information|GetAffectedObjects) true))
                    (:Backward
                      ;[1 1 1] Beginning of Transition, Appear/Disappear Actors
                      (for _array_element (Variables|Parameters|GetTransitionToggleList)
                        (Default|ExitTransition _array_element)))))))
            (:then_1
              (Rendering|SetActorHiddenInGame (Variables|Information|GetAffectedObjects) false))))))
    (:then_1
      (Utilities|FlowControl|DoOnce false) ; enters at Reset
    )))

(event Custom|ResetLight
  ;[1 1 1] Work around Issue with Already Overlapping Objects not triggering "Begin Overlap".
  (for _array_element (Collision|GetOverlappingActors (Variables|Default|GetSphereCollider) 0 :!class /Script/Engine.PrimitiveComponent)
    (CallFunction|OnLightBeginOverlap _array_element)))

(event Custom|OnLightEndOverlap
  (params (OtherActor :type Actor%20Object%20Reference) (OtherComp :type Primitive%20Component%20Object%20Reference))
  (bind _returnvalue (Actor|GetComponentbyClass OtherActor "/Game/Environment/Interactable/LampOfAlhazred/Blueprints/BP_MaterialTransformComponent.BP_MaterialTransformComponent_C"))
  (Utilities|IsValid _returnvalue
    (:Is%20Valid
      (Default|RemoveLitObject (Variables|Default|GetTransitionManagerRef) _returnvalue)
      (Utilities|Array|RemoveItem (Variables|Default|GetLitObjectList) _returnvalue))))

(event EventBeginPlay
  (CallFunction|RetrieveTransitionManager)
  (Components|Timeline|SetPlayRate (Variables|Default|GetTransitionTimeline) (/ 1.0 (Variables|Default|GetTransitionSpeed)))
  (Variables|Default|SetInitialLightRadius (Variables|Parameters|GetLightRadius))
  (CallFunction|UpdateProperties 0.0)
  (Default|ClearLitObjects (Variables|Default|GetTransitionManagerRef)))

(event EventTick
  (params (DeltaSeconds :type Float%20%28single-precision%29))
  (CallFunction|UpdatePositionPrivate))

(fn ConstructionScript
  (bind _spherecollider (Variables|Default|GetSphereCollider))
  (bind _debugcenter (Variables|Default|GetDebugCenter))
  (bind _lightradius (Variables|Parameters|GetLightRadius))
  (Utilities|FlowControl|Sequence
    (:then_0
      (Components|Sphere|SetSphereRadius (Variables|Default|GetSphereCollider) (* (Variables|Parameters|GetLightRadius) (Variables|Default|GetWorldToColliderUnit)) false)
      (if (Variables|Parameters|GetIsDebugCenterActive)
        (Transformation|SetWorldScale3D _debugcenter (Math|Vector|MakeVector _lightradius _lightradius _lightradius))
        (else
          (Transformation|SetWorldScale3D _debugcenter (Math|Vector|MakeVector 0.1 0.1 0.1)))))
    (:then_1
      (Collision|SetCollisionEnabled _spherecollider "QueryOnly")
      (bind _outactors (Class|KismetSystemLibrary|ComponentOverlapActorsNEW _spherecollider (Transformation|GetWorldTransform _spherecollider) (Utilities|Array|MakeArray "ObjectTypeQuery1") "/Script/Engine.Actor" (Variables|Parameters|GetUnaffectedObjectList)))
      (bind _newparam (CallFunction|FilterActorsbyComponent _outactors "/Game/Environment/Interactable/LampOfAlhazred/Blueprints/BP_MaterialTransformComponent.BP_MaterialTransformComponent_C"))
      (Variables|Information|SetAffectedObjects _newparam)
      (Collision|SetCollisionEnabled _spherecollider "NoCollision"))))

(fn UpdatePositionPrivate
  (if (> (Variables|Parameters|GetLightRadius) 0.0)
    (bind _output_get (LocalVariables|SetCurrentLocation (Transformation|GetWorldLocation (Variables|Default|GetRoot))))
    (if (Math|Vector|NotEqual(Vector) _output_get (Variables|Default|GetSpherePosition) 0.0001)
      (Variables|Default|SetSpherePosition (LocalVariables|GetCurrentLocation))
      (for _array_element (Variables|Default|GetLitObjectList)
        (Default|UpdateSpherePosition _array_element (Variables|Default|GetSpherePosition) (Variables|Parameters|GetLightIndex))))))

(fn UpdateRadius
  (params (Radius :type Float%20%28single-precision%29))
  (Variables|Parameters|SetLightRadius Radius)
  (CallFunction|UpdateColliderPrivate)
  (for _array_element (Variables|Default|GetLitObjectList)
    (Default|UpdateSphereRadius _array_element Radius (Variables|Parameters|GetLightIndex))))

(fn UpdateProperties
  (params (Radius :type Float%20%28single-precision%29))
  (Variables|Parameters|SetLightRadius Radius)
  (CallFunction|UpdateColliderPrivate)
  (for _array_element (Variables|Default|GetLitObjectList)
    (Default|UpdateSphereProperties _array_element Radius (Variables|Parameters|GetLightIndex))))

(fn UpdateColliderPrivate
  (Collision|SetCollisionEnabled (Variables|Default|GetSphereCollider) (select (Math|Float|NearlyEqual(Float) (Variables|Parameters|GetLightRadius) 0.0 0.001) "NoCollision" "QueryOnly"))
  (Components|Sphere|SetSphereRadius (Variables|Default|GetSphereCollider) (* (Variables|Parameters|GetLightRadius) (Variables|Default|GetWorldToColliderUnit)) true))

(fn GetRadius
  (return (Variables|Parameters|GetLightRadius)))

(fn GetIndex
  (return (Variables|Parameters|GetLightIndex)))

(fn RetrieveTransitionManager
  (bind _asbp_transition_manager (Utilities|Casting|CastToBP_TransitionManager (Components|GetOwner (Transformation|GetAttachParent (Variables|Default|GetRoot))))
    (:then
      (bind _output_get (Variables|Default|SetTransitionManagerRef _asbp_transition_manager))
      (Default|AddTransitionSphere _output_get self))
    (:CastFailed
      (Development|PrintString "FEHFVKEJWGFCHJ" true true "(R=0.000000,G=0.660000,B=1.000000,A=1.000000)" 2e+01))))