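; Manager for the Lamp of Alhazred's transition spheres, tracking the objects they light and feeding sphere data to those objects' materials.
; It keeps a unique sphere list plus parallel arrays of lit objects and reference counts, so overlapping spheres share one entry.
; Adding pushes sphere position, radius and index, initializing detection on first entry.
; Detection is uninitialized when the last reference is removed or the list is cleared.
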(event Collision|EventActorBeginOverlap
  (params (OtherActor :type Actor%20Object%20Reference)))

(event EventTick
  (params (DeltaSeconds :type Float%20%28single-precision%29)))

(fn ConstructionScript)

(fn AddTransitionSphere
  (params (Sphere :type BP%20Transition%20Sphere%20Object%20Reference))
  (Utilities|Array|AddUnique (Variables|Default|GetTransitionSphereList) Sphere))

(fn AddLitObject
  (params (Sphere :type BP%20Transition%20Sphere%20Object%20Reference) (Material :type BP%20Material%20Transform%20Component%20Object%20Reference))
  (bind _litobjrefcountlist (Variables|Default|GetLitObjRefCountList))
  (LocalVariables|SetIndexFound -1)
  (Default|UpdateSpherePosition Material (Transformation|GetActorLocation Sphere) (Default|GetIndex Sphere))
  (bind (_array_element _array_index) (Utilities|Array|ForEachLoopwithBreak (Variables|Default|GetLitObjectList) :!label _label)
    (:LoopBody
      (if (== Material _array_element)
        (LocalVariables|SetIndexFound _array_index)
        (goto _label Break)))
    (:Completed
      (if (== (LocalVariables|GetIndexFound) -1)
        (Utilities|Array|Add (Variables|Default|GetLitObjectList) Material)
        (Utilities|Array|Add (Variables|Default|GetLitObjRefCountList) 1)
        (Default|InitializeSphereDetection Material (Default|GetRadius Sphere) (Default|GetIndex Sphere))
        (else
          (Utilities|Array|SetArrayElem _litobjrefcountlist (LocalVariables|GetIndexFound) (+ (Utilities|Array|Get(acopy) _litobjrefcountlist (LocalVariables|GetIndexFound)) 1))
          (Default|UpdateSphereProperties Material (Default|GetRadius Sphere) (Default|GetIndex Sphere)))))))

(fn RemoveLitObject
  (params (Material :type BP%20Material%20Transform%20Component%20Object%20Reference))
  (bind _returnvalue (Utilities|String|MakeLiteralString "THIS SHOULD NOT TRIGGER!"))
  (bind _litobjrefcountlist (Variables|Default|GetLitObjRefCountList))
  (LocalVariables|SetIndexFound -1)
  (bind (_array_element _array_index) (Utilities|Array|ForEachLoopwithBreak (Variables|Default|GetLitObjectList) :!label _label)
    (:LoopBody
      (if (== Material _array_element)
        (LocalVariables|SetIndexFound _array_index)
        (goto _label Break)))
    (:Completed
      (if (>= (LocalVariables|GetIndexFound) 0)
        (if (<= (Utilities|Array|Get(acopy) _litobjrefcountlist (LocalVariables|GetIndexFound)) 1)
          (Utilities|Array|RemoveIndex (Variables|Default|GetLitObjectList) (LocalVariables|GetIndexFound))
          (Utilities|Array|RemoveIndex (Variables|Default|GetLitObjRefCountList) (LocalVariables|GetIndexFound))
          (Default|UninitializeSphereDetection Material)
          (else
            (Utilities|Array|SetArrayElem _litobjrefcountlist (LocalVariables|GetIndexFound) (- (Utilities|Array|Get(acopy) _litobjrefcountlist (LocalVariables|GetIndexFound)) 1))))
        (else
          (Development|PrintString _returnvalue true false "(R=1.000000,G=0.000000,B=0.000000,A=1.000000)" 2e+01)
          (CallFunction|PrintMessage _returnvalue 2e+01 "(R=1.000000,G=0.000000,B=0.000000,A=1.000000)"))))))

(fn ClearLitObjects
  (bind _litobjectlist (Variables|Default|GetLitObjectList))
  (bind _litobjrefcountlist (Variables|Default|GetLitObjRefCountList))
  (for _array_element (Variables|Default|GetLitObjectList)
    (Default|UninitializeSphereDetection _array_element))
  (Utilities|Array|Clear _litobjectlist)
  (Utilities|Array|Resize _litobjectlist 0)
  (Utilities|Array|Clear _litobjrefcountlist)
  (Utilities|Array|Resize _litobjrefcountlist 0))