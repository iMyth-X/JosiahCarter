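; BP_LampOfAlhazred_Artifact is the interactable Lamp of Alhazred artifact, which triggers a world transition when used.
; A DoOnce on interaction begin has the game manager, reached through the VR game instance, play the activation sound, then fires the flameburst particle.
; Timed delays start the transition shortly after the burst and later switch the particle off.
; GetArtifactColor supplies yellow as the artifact's color.
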(event EventBeginPlay
  (|CallParentFunction))

(event Collision|EventActorBeginOverlap
  (params (OtherActor :type Actor%20Object%20Reference)))

(event EventTick
  (params (DeltaSeconds :type Float%20%28single-precision%29)))

(event EventOnInteractionBegin
  (params (SilverKey :type BP%20Silver%20Key%20Object%20Reference))
  (bind _flameburstparticle (Variables|Default|GetFlameburstParticle))
  (Utilities|FlowControl|DoOnce false
    (:Completed
      (bind _asmy_vrgame_instance_bp (Utilities|Casting|CastToMyVRGameInstanceBP (Game|GetGameInstance)))
      (Default|PlayLampActivationSound (Default|GetGameManager _asmy_vrgame_instance_bp))
      (Components|Activation|Activate _flameburstparticle false)
      (Utilities|FlowControl|Delay 2.0)
      (CallFunction|StartWorldTransition)
      (Utilities|FlowControl|Delay 5.0)
      (Components|Activation|Deactivate _flameburstparticle))))

(fn ConstructionScript
  (|CallParentFunction))

(fn GetArtifactColor
  (return "(R=1.000000,G=1.000000,B=0.000000,A=1.000000)"))