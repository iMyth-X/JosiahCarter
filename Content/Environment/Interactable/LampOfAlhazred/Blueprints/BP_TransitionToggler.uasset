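; BP_TransitionToggler switches two actor lists, World A and World B, between visible and hidden as a Lamp of Alhazred transition is entered or exited.
; EnterTransition and ExitTransition adjust a counter, so World B stays shown until nested entries have all exited.
; A shared private function sets hidden-in-game and propagated root visibility oppositely per list.
; The construction script applies StartWorldA; its logic restoring objects removed from the lists is disconnected.
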(event EventBeginPlay)

(event Collision|EventActorBeginOverlap
  (params (OtherActor :type Actor%20Object%20Reference)))

(event EventTick
  (params (DeltaSeconds :type Float%20%28single-precision%29)))

(fn ConstructionScript
  (CallFunction|SetTransitionStatePRIVATE (not (Variables|Parameters|GetStartWorldA))))

(fn EnterTransition
  (bind _result (Math|Integer|IncrementInt (Variables|Default|GetEnteredTransitionCount))
    (:%20%20
      (if (> _result 0)
        (CallFunction|SetTransitionStatePRIVATE true)))))

(fn ExitTransition
  (bind _result (Math|Integer|DecrementInt (Variables|Default|GetEnteredTransitionCount))
    (:%20%20
      (if (<= _result 0)
        (CallFunction|SetTransitionStatePRIVATE false)))))

(fn SetTransitionStatePRIVATE
  (params (HasEnteredTransition :type Boolean))
  (bind _returnvalue (not HasEnteredTransition))
  (bind _worldaobjects (Variables|Parameters|GetWorldAObjects))
  (bind _worldbobjects (Variables|Parameters|GetWorldBObjects))
  (Utilities|FlowControl|Sequence
    (:then_0
      (Rendering|SetActorHiddenInGame _worldaobjects HasEnteredTransition)
      (for _array_element _worldaobjects
        (Rendering|SetVisibility (VehicleSound|GetRootComponent _array_element) _returnvalue true)))
    (:then_1
      (Rendering|SetActorHiddenInGame _worldbobjects _returnvalue)
      (for _array_element_2 _worldbobjects
        (Rendering|SetVisibility (VehicleSound|GetRootComponent _array_element_2) HasEnteredTransition true)))))