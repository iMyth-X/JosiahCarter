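; Material transform component for Lamp of Alhazred interactables, swapping meshes between normal and dimensional materials while sphere detection is active.
; Builds paired dynamic materials from texture buffers, choosing transparent or normal parents, and assigns them to listed mesh slots by clamped index.
; Indexed sphere center and scaled radius parameters drive the dimensional materials.
; Uninitializing, also run at BeginPlay, zeroes three sphere radii and restores normal materials.
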(event EventBeginPlay
  (|CallParentFunction)
  (CallFunction|UninitializeSphereDetection))

(event EventClearMaterialLists
  (Utilities|Array|Clear (Variables|Default|GetNormalMaterialList))
  (Utilities|Array|Clear (Variables|Default|GetDimensionalMaterialList)))

(event EventConstructionScript
  (|CallParentFunction))

(fn UpdateSpherePosition
  (params (CenterPosition :type Vector) (Index :type Integer))
  (LocalVariables|SetCenterPositionTag (Utilities|String|StringToName (Utilities|String|Append "CenterPosition" (Utilities|String|ToString(Integer) Index))))
  (for _array_element (Variables|Default|GetDimensionalMaterialList)
    (Rendering|Material|SetVectorParameterValue _array_element (LocalVariables|GetCenterPositionTag) (Math|Conversions|ToLinearColor(Vector) CenterPosition) :!class /Script/Engine.MaterialInstanceDynamic)))

(fn InitializeSphereDetection
  (params (Radius :type Float%20%28single-precision%29) (Index :type Integer))
  (bind _dimensionalmateriallist (Variables|Default|GetDimensionalMaterialList))
  (CallFunction|UpdateSphereProperties Radius Index)
  (Default|CallOnMaterialTransform)
  ;[1 1 1] Replace the Normal Material with the Transforming Material
  (for (_array_element _array_index) (Variables|Default|GetMeshInfoList)
    (Rendering|Material|SetMaterial (.mesh _array_element) (.materialindex _array_element) (Utilities|Array|Get(acopy) _dimensionalmateriallist (Math|Integer|Clamp(Integer) _array_index 0 (Utilities|Array|LastIndex _dimensionalmateriallist))))))

(fn UpdateSphereRadius
  (params (Radius :type Float%20%28single-precision%29) (Index :type Integer))
  (LocalVariables|SetRadiusTag (Utilities|String|StringToName (Utilities|String|Append "Radius" (Utilities|String|ToString(Integer) Index))))
  (for _array_element (Variables|Default|GetDimensionalMaterialList)
    (Rendering|Material|SetScalarParameterValue _array_element (LocalVariables|GetRadiusTag) (* Radius (Variables|Default|GetWorldToMaskUnit)) :!class /Script/Engine.MaterialInstanceDynamic)))

(fn UninitializeSphereDetection
  (bind _normalmateriallist (Variables|Default|GetNormalMaterialList))
  ;[1 1 1] Reset Sphere Properties to 0
  (bind _index (Utilities|ForLoop(Fixed) 0 2)
    (:Completed
      (Default|CallOnMaterialUntransform)
      ;[1 1 1] Return the Transforming Material to its Normal Material State
      (for (_array_element _array_index) (Variables|Default|GetMeshInfoList)
        (Rendering|Material|SetMaterial (.mesh _array_element) (.materialindex _array_element) (Utilities|Array|Get(acopy) _normalmateriallist (Math|Integer|Clamp(Integer) _array_index 0 (Utilities|Array|LastIndex _normalmateriallist))))))
    (:LoopBody
      (CallFunction|UpdateSphereProperties 0.0 _index))))

(fn UpdateSphereProperties
  (params (Radius :type Float%20%28single-precision%29) (Index :type Integer))
  (CallFunction|UpdateSphereRadius Radius Index))

(fn InitializeMaterialListElementsfromTextureBuffer
  (params (TextureBuffer :type Texture%20Buffer%20Structure%20%28by%20ref%29))
  (if (.bIsTransparent (Utilities|Struct|BreakTextureBuffer TextureBuffer))
    (bind _dynamicmaterial (CallFunction|CreateMaterialDynamic "/Game/Environment/Interactable/LampOfAlhazred/Materials/M_TransparentDimensionalMaterial.M_TransparentDimensionalMaterial" TextureBuffer))
    (LocalVariables|SetDimensionalMaterial _dynamicmaterial)
    (bind _dynamicmaterial_2 (CallFunction|CreateMaterialDynamic "/Game/Environment/Interactable/LampOfAlhazred/Materials/M_TransparentMaterial.M_TransparentMaterial" TextureBuffer))
    (LocalVariables|SetNormalMaterial _dynamicmaterial_2)
    (else
      (bind _dynamicmaterial_3 (CallFunction|CreateMaterialDynamic "/Game/Environment/Interactable/LampOfAlhazred/Materials/M_NormalDimensionalMaterial.M_NormalDimensionalMaterial" TextureBuffer))
      (LocalVariables|SetDimensionalMaterial _dynamicmaterial_3)
      (bind _dynamicmaterial_4 (CallFunction|CreateMaterialDynamic "/Game/Environment/Interactable/LampOfAlhazred/Materials/M_NormalMaterial.M_NormalMaterial" TextureBuffer))
      (LocalVariables|SetNormalMaterial _dynamicmaterial_4)))
  (Utilities|Array|Add (Variables|Default|GetDimensionalMaterialList) (LocalVariables|GetDimensionalMaterial))
  (Utilities|Array|Add (Variables|Default|GetNormalMaterialList) (LocalVariables|GetNormalMaterial))
  (return (LocalVariables|GetNormalMaterial)))