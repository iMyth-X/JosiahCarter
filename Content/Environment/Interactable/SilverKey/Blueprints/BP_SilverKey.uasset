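; Silver Key interactable that reacts to artifacts overlapping its capsule and is revealed from a child-actor courier box that it detaches and opens.
; It tracks overlapping artifacts, keeps one in focus to receive begin, per-tick hit and end interaction calls, and falls back to another on exit.
; A timeline blends its emissive glow toward the focused artifact's colour, then signals completion once after three distinct artifacts have been interacted with.
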(event OnComponentBeginOverlap(Capsule)
  (params (OverlappedComponent :type Primitive%20Component%20Object%20Reference) (OtherActor :type Actor%20Object%20Reference) (OtherComp :type Primitive%20Component%20Object%20Reference) (OtherBodyIndex :type Integer) (bFromSweep :type Boolean) (SweepResult :type Hit%20Result%20Structure%20%28by%20ref%29))
  ;[1 1 1] On Artifact Begin Overlap
  (bind _asbp_abstract_artifact (Utilities|Casting|CastToBP_AbstractArtifact OtherActor))
  (CallFunction|OnArtifactBeginOverlap _asbp_abstract_artifact))

(event OnComponentEndOverlap(Capsule)
  (params (OverlappedComponent :type Primitive%20Component%20Object%20Reference) (OtherActor :type Actor%20Object%20Reference) (OtherComp :type Primitive%20Component%20Object%20Reference) (OtherBodyIndex :type Integer))
  ;[1 1 1] On Artifact End Overlap
  (bind _asbp_abstract_artifact (Utilities|Casting|CastToBP_AbstractArtifact OtherActor))
  (CallFunction|OnArtifactEndOverlap _asbp_abstract_artifact))

(event Custom|OnArtifactBeginOverlap
  (params (Artifact :type BP%20Abstract%20Artifact%20Object%20Reference))
  ;[1 1 1] On Artifact Begin Overlap
  (if (!= (Variables|Default|GetFocusArtifact) Artifact)
    (Utilities|Array|AddUnique (Variables|Default|GetArtifactList) Artifact)
    (Utilities|FlowControl|Sequence
      (:then_0
        (Utilities|IsValid (Variables|Default|GetFocusArtifact)
          (:Is%20Valid
            (CallFunction|OnArtifactEndOverlap (Variables|Default|GetFocusArtifact)))
          (:Is%20Not%20Valid
            (bind _emissivecolor (Default|GetArtifactColor Artifact))
            (Variables|Default|SetEmissiveColor _emissivecolor))))
      (:then_1
        (bind _output_get (Variables|Default|SetFocusArtifact Artifact))
        (CallFunction|OnArtifactInteractionBegin _output_get)))))

(event Custom|DetachFromCourierBox
  (bind _returnvalue (Math|Float|MakeLiteralFloat 4.0))
  (bind _courierbox (Variables|Default|GetCourierBox))
  (Transformation|DetachFromActor _courierbox "KeepWorld" "KeepWorld" "KeepWorld")
  ;[1 1 1] Again! Because why not?
  (Transformation|DetachFromActor _courierbox "KeepWorld" "KeepWorld" "KeepWorld")
  (Default|OpenBox _courierbox _returnvalue)
  (Utilities|FlowControl|Delay (/ _returnvalue 4.0))
  (Rendering|SetVisibility (Variables|Default|GetSilverKey) true false))

(event Custom|OnArtifactEndOverlap
  (params (Artifact :type BP%20Abstract%20Artifact%20Object%20Reference))
  (bind _artifactlist (Variables|Default|GetArtifactList))
  ;[1 1 1] On Artifact End Overlap
  (Utilities|Array|RemoveItem _artifactlist Artifact)
  (if (== Artifact (Variables|Default|GetFocusArtifact))
    (CallFunction|OnArtifactInteractionEnd (Variables|Default|GetFocusArtifact))
    (if (>= (Utilities|Array|LastIndex _artifactlist) 0)
      (bind _output_get (Variables|Default|SetFocusArtifact (Utilities|Array|Get(acopy) _artifactlist)))
      (CallFunction|OnArtifactInteractionBegin _output_get)
      (else
        (Variables|Default|SetFocusArtifact 0)
        (CallFunction|StopEmissiveGlow)))))

(event Custom|OnArtifactInteractionBegin
  (params (Artifact :type BP%20Abstract%20Artifact%20Object%20Reference))
  ;[1 1 1] Silver Key Begin Artifact Interaction
  (Default|OnInteractionBegin Artifact self)
  (Default|StartEmissiveGlow Artifact)
  (CallFunction|StartEmissiveGlow)
  (Utilities|Array|AddUnique (Variables|Default|GetArtifactInteractedList) Artifact))

(event Custom|OnArtifactInteractionEnd
  (params (Artifact :type BP%20Abstract%20Artifact%20Object%20Reference))
  ;[1 1 1] Silver Key End Artifact Interaction
  (Default|OnInteractionEnd Artifact self)
  (Default|StopEmissiveGlow Artifact))

(event Custom|StartEmissiveGlow
  (bind _focusartifact (Variables|Default|GetFocusArtifact))
  ;[1 1 1] Silver Key Glow Effect
  (Variables|Default|SetPreviousEmissiveColor (Variables|Default|GetEmissiveColor))
  (Variables|Default|SetPreviousEmissiveIntensity (Variables|Default|GetEmissiveIntensity))
  (bind (_direction _gradient) (Timeline|ArtifactTransition PlayFromStart)
    (:Update
      (Utilities|FlowControl|Sequence
        (:then_0
          (Utilities|IsValid _focusartifact
            (:Is%20Valid
              (bind _emissivecolor (Default|GetArtifactColor _focusartifact))
              (bind _output_get (Variables|Default|SetEmissiveColor (Math|Color|Lerp(LinearColor) (Variables|Default|GetPreviousEmissiveColor) _emissivecolor _gradient)))
              (Default|SetEmissiveColor (Variables|Default|GetBP_MaterialGlowComponent) _output_get))))
        (:then_1
          (switch Utilities|FlowControl|Switch|SwitchonETimelineDirection _direction
            (:Forward
              (Variables|Default|SetEmissiveIntensity (Math|Float|Lerp (Variables|Default|GetPreviousEmissiveIntensity) 1.0 _gradient)))
            (:Backward
              (Variables|Default|SetEmissiveIntensity (Math|Float|Lerp 0.0 (Variables|Default|GetPreviousEmissiveIntensity) _gradient))))
          (Default|SetEmissiveIntensity (Variables|Default|GetBP_MaterialGlowComponent) (* (Variables|Default|GetEmissiveIntensity) (Math|Float|MakeLiteralFloat 0.05))))))
    (:Finished
      ;;[1 1 1] Check End Condition (All 3 Artifacts have been interacted with)
      (Utilities|FlowControl|Delay 5.0)
      (if (>= (Utilities|Array|Length (Variables|Default|GetArtifactInteractedList)) 3)
        (Utilities|FlowControl|DoOnce false
          (:Completed
            (Default|CallSilverKeyInteractionComplete)))))))

(event Custom|StopEmissiveGlow
  (bind _focusartifact (Variables|Default|GetFocusArtifact))
  ;[1 1 1] Silver Key Glow Effect
  (Variables|Default|SetPreviousEmissiveColor (Variables|Default|GetEmissiveColor))
  (Variables|Default|SetPreviousEmissiveIntensity (Variables|Default|GetEmissiveIntensity))
  (bind (_direction _gradient) (Timeline|ArtifactTransition ReverseFromEnd)
    (:Update
      (Utilities|FlowControl|Sequence
        (:then_0
          (Utilities|IsValid _focusartifact
            (:Is%20Valid
              (bind _emissivecolor (Default|GetArtifactColor _focusartifact))
              (bind _output_get (Variables|Default|SetEmissiveColor (Math|Color|Lerp(LinearColor) (Variables|Default|GetPreviousEmissiveColor) _emissivecolor _gradient)))
              (Default|SetEmissiveColor (Variables|Default|GetBP_MaterialGlowComponent) _output_get))))
        (:then_1
          (switch Utilities|FlowControl|Switch|SwitchonETimelineDirection _direction
            (:Forward
              (Variables|Default|SetEmissiveIntensity (Math|Float|Lerp (Variables|Default|GetPreviousEmissiveIntensity) 1.0 _gradient)))
            (:Backward
              (Variables|Default|SetEmissiveIntensity (Math|Float|Lerp 0.0 (Variables|Default|GetPreviousEmissiveIntensity) _gradient))))
          (Default|SetEmissiveIntensity (Variables|Default|GetBP_MaterialGlowComponent) (* (Variables|Default|GetEmissiveIntensity) (Math|Float|MakeLiteralFloat 0.05))))))
    (:Finished
      ;;[1 1 1] Check End Condition (All 3 Artifacts have been interacted with)
      (Utilities|FlowControl|Delay 5.0)
      (if (>= (Utilities|Array|Length (Variables|Default|GetArtifactInteractedList)) 3)
        (Utilities|FlowControl|DoOnce false
          (:Completed
            (Default|CallSilverKeyInteractionComplete)))))))

(event Custom|Activate
  ;[1 1 1] Activate the Silver Key
  (Collision|SetCollisionEnabled (Variables|Default|GetCapsule) "QueryOnly"))

(event EventBeginPlay
  ;[1 1 1] On Begin Play Overlap
  (for _array_element (Collision|GetOverlappingActors (Variables|Default|GetCapsule) 0 :!class /Script/Engine.PrimitiveComponent)
    (bind _asbp_abstract_artifact (Utilities|Casting|CastToBP_AbstractArtifact _array_element))
    (CallFunction|OnArtifactBeginOverlap _asbp_abstract_artifact)
    ;[1 1 1] How Long the Color Transition Should Take
    (Components|Timeline|SetPlayRate (Variables|Default|GetArtifactTransition) 1.0)
    (Collision|SetCollisionEnabled (Variables|Default|GetCapsule) "NoCollision")))

(event EventTick
  (params (DeltaSeconds :type Float%20%28single-precision%29))
  (bind _focusartifact (Variables|Default|GetFocusArtifact))
  ;[1 1 1] On Artifact Hit
  (Utilities|IsValid _focusartifact
    (:Is%20Valid
      (Default|OnInteractionHit _focusartifact self))))

(fn ConstructionScript
  (|CallParentFunction)
  ;[1 1 1] Get Courier Box
  (bind _asbp_courier_box_final (Utilities|Casting|CastToBP_CourierBoxFinal (Variables|/Script/Engine.ChildActorComponent|GetChildActor (Variables|Default|GetCourierBoxActor))))
  (Variables|Default|SetCourierBox _asbp_courier_box_final))

(fn SetVibrationIntensity
  (params (Intensity :type Float%20%28single-precision%29) (Duration :type Float%20%28single-precision%29)))