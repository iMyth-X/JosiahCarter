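; BP_FrontDoor is a front door with two leaves that swing open and closed on command.
; OpenDoor, CloseDoor and StopDoor play, reverse or stop one timeline, setting opening and reversing flags.
; The timeline sets mirrored world-space yaw, always on the right leaf and on the left only when OpenBoth is true.
; On finish, its direction selects the opened or closed notification; a creak-sound debug print is left unconnected.
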(event Custom|OpenDoor
  ;[1 1 1] Door Rotation
  (Variables|Default|SetbIsOpening true)
  (bind (_direction _door_movement) (Timeline|Door%20Timeline Play)
    (:Update
      (Utilities|FlowControl|Sequence
        (:then_0
          (if (Variables|Default|GetbOpenBoth)
            (Transformation|SetWorldRotation (Variables|Default|GetDoorLeft) (Math|Rotator|MakeRotator 0.0 0.0 _door_movement) false false)))
        (:then_1
          (Transformation|SetWorldRotation (Variables|Default|GetDoorRight) (Math|Rotator|MakeRotator 0.0 0.0 (- 1.8e+02 _door_movement)) false false))))
    (:Finished
      (switch Utilities|FlowControl|Switch|SwitchonETimelineDirection _direction
        (:Forward
          (Default|CallOnDoorOpened))
        (:Backward
          (Default|CallOnDoorClosed))))))

(event Custom|StopDoor
  ;[1 1 1] Door Rotation
  (Variables|Default|SetbIsOpening false)
  (Variables|Default|SetbIsReversing false)
  (bind (_direction _door_movement) (Timeline|Door%20Timeline Stop)
    (:Update
      (Utilities|FlowControl|Sequence
        (:then_0
          (if (Variables|Default|GetbOpenBoth)
            (Transformation|SetWorldRotation (Variables|Default|GetDoorLeft) (Math|Rotator|MakeRotator 0.0 0.0 _door_movement) false false)))
        (:then_1
          (Transformation|SetWorldRotation (Variables|Default|GetDoorRight) (Math|Rotator|MakeRotator 0.0 0.0 (- 1.8e+02 _door_movement)) false false))))
    (:Finished
      (switch Utilities|FlowControl|Switch|SwitchonETimelineDirection _direction
        (:Forward
          (Default|CallOnDoorOpened))
        (:Backward
          (Default|CallOnDoorClosed))))))

(event Custom|CloseDoor
  ;[1 1 1] Door Rotation
  (Variables|Default|SetbIsReversing true)
  (bind (_direction _door_movement) (Timeline|Door%20Timeline Reverse)
    (:Update
      (Utilities|FlowControl|Sequence
        (:then_0
          (if (Variables|Default|GetbOpenBoth)
            (Transformation|SetWorldRotation (Variables|Default|GetDoorLeft) (Math|Rotator|MakeRotator 0.0 0.0 _door_movement) false false)))
        (:then_1
          (Transformation|SetWorldRotation (Variables|Default|GetDoorRight) (Math|Rotator|MakeRotator 0.0 0.0 (- 1.8e+02 _door_movement)) false false))))
    (:Finished
      (switch Utilities|FlowControl|Switch|SwitchonETimelineDirection _direction
        (:Forward
          (Default|CallOnDoorOpened))
        (:Backward
          (Default|CallOnDoorClosed))))))

(fn ConstructionScript
  (|CallParentFunction))