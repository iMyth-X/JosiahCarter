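; Elevator actor that descends from its placed height to a fixed floor height, firing begin and end events and opening its sliding doors on arrival.
; Timelines drive the descent, the door slide and a duration-scaled cabin shake.
; UpdateElevatorTotalTime retimes the descent mid-ride by tracking playback position and rescaling the timeline's play rate.
; EndElevatorTime converts a requested time left into a new total, with debug prints checking timing.
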(event Custom|BeginElevatorDescent
  (bind _returnvalue (Utilities|Time|GetGameTimeinSeconds))
  (Utilities|FlowControl|Sequence
    (:then_0
      (Variables|Default|SetElevatorStartTime _returnvalue)
      (Default|CallOnElevatorBeginDescent)
      (bind _elevatormovement (Timeline|ElevatorMovement Play)
        (:Update
          (Transformation|SetActorLocation (Math|Vector|MakeVector (Variables|Default|GetOriginalLocationX) (Variables|Default|GetOriginalLocationY) (- (Variables|Default|GetOriginalLocationZ) (* _elevatormovement (Variables|Default|GetFloorOffset)))) false false))
        (:Finished
          (Default|CallOnElevatorEndDescent)
          (CallFunction|SetDoorState true)
          ;[1 1 1] DEBUG
          (if (Variables|Parameters|GetbIsInDebugMode)
            (Development|PrintString (Utilities|String|Append "Complete at " (Utilities|String|ToString(Float) (Utilities|Time|GetGameTimeinSeconds))) true true "(R=0.000000,G=1.000000,B=0.051031,A=1.000000)" 1e+02)))))
    (:then_1
      ;[1 1 1] DEBUG
      (if (Variables|Parameters|GetbIsInDebugMode)
        (Development|PrintString (Utilities|String|Append "Elevator Beginning at " (Utilities|String|ToString(Float) _returnvalue)) true true "(R=0.000000,G=1.000000,B=0.051031,A=1.000000)" 1e+02)))))

(event Custom|ShakeElevator
  (params (Duration :type Float%20%28single-precision%29))
  (Components|Timeline|SetPlayRate (Variables|Default|GetElevatorShakeTimeline) (/ 1.0 Duration))
  (bind (_direction _shakeinroll _shakeinpitch _shakeinyaw) (Timeline|ElevatorShakeTimeline PlayFromStart)
    (:Update
      (Transformation|SetRelativeRotation (Variables|Default|GetElevator) (Math|Rotator|MakeRotator _shakeinroll _shakeinpitch _shakeinyaw) false false))))

(event Custom|SetDoorState
  (params (Open? :type Boolean))
  (bind _sm_elevator_rightdoor (Variables|Default|GetSM_Elevator_RightDoor))
  (bind _sm_elevator_leftdoor (Variables|Default|GetSM_Elevator_LeftDoor))
  (bind _relativelocation (Variables|/Script/Engine.SceneComponent|GetRelativeLocation _sm_elevator_leftdoor))
  (bind _relativelocation_2 (Variables|/Script/Engine.SceneComponent|GetRelativeLocation _sm_elevator_rightdoor))
  (bind (_x _y _z) (Math|Vector|BreakVector _relativelocation))
  (bind (_x_2 _y_2 _z_2) (Math|Vector|BreakVector _relativelocation_2))
  ;[1 1 1] Door Opening Animation
  (Components|Timeline|SetPlayRate (Variables|Default|GetElevatorDoorAnim) (Variables|Default|GetDoorOpenSpeed))
  (if Open?
    (bind _x_3 (Timeline|Elevator_DoorAnim PlayFromStart)
      (:Update
        (Transformation|SetRelativeLocationAndRotation _sm_elevator_leftdoor (Math|Vector|MakeVector _x_3 _y _z) "0.000000,0.000000,0.000000" false false)
        (Transformation|SetRelativeLocationAndRotation (Variables|Default|GetSM_Elevator_RightDoor) (Math|Vector|MakeVector (* _x_3 -1.0) _y_2 _z_2) "0.000000,0.000000,0.000000" false false)))
    (else
      (Timeline|Elevator_DoorAnim ReverseFromEnd))))

(event EventBeginPlay
  (bind _returnvalue (Transformation|GetActorLocation))
  (bind (_x _y _z) (Math|Vector|BreakVector _returnvalue))
  (Variables|Default|SetOriginalLocationX _x)
  (Variables|Default|SetOriginalLocationY _y)
  (bind _output_get (Variables|Default|SetOriginalLocationZ _z))
  (bind _output_get_2 (Variables|Default|SetFinalLocationZ 4e+01))
  (Variables|Default|SetFloorOffset (- _output_get _output_get_2)))

(fn ConstructionScript)

(fn UpdateElevatorTotalTime
  (params (TimeInSeconds :type Float%20%28single-precision%29))
  (LocalVariables|SetNewTotalTime TimeInSeconds)
  (Utilities|FlowControl|Sequence
    (:then_0
      (bind _output_get (LocalVariables|SetCurrentPlaybackPosition (Components|Timeline|GetPlaybackPosition (Variables|Default|GetElevatorMovement))))
      (Variables|Default|SetElevatorCurrentTime (+ (Variables|Default|GetElevatorCurrentTime) (* (- _output_get (Variables|Default|GetPreviousPlaybackPosition)) (Variables|Default|GetElevatorPlayRate))))
      (Variables|Default|SetPreviousPlaybackPosition (LocalVariables|GetCurrentPlaybackPosition)))
    (:then_1
      (bind _output_get_2 (LocalVariables|SetTotalTimeDifference (- (Variables|Parameters|GetElevatorTotalTime) (Variables|Default|GetElevatorCurrentTime))))
      (if (< _output_get_2 0.0)
        (return)))
    (:then_2
      (bind _output_get_3 (LocalVariables|SetNewTotalTimeDifference (- (LocalVariables|GetNewTotalTime) (Variables|Default|GetElevatorCurrentTime))))
      (if (< _output_get_3 0.0)
        (return)
        (else
          (Variables|Parameters|SetElevatorTotalTime (LocalVariables|GetNewTotalTime))
          (if (Variables|Parameters|GetbIsInDebugMode)
            ;[1 1 1] DEBUG
            (if (Math|Float|NearlyEqual(Float) (/ 1.0 (Variables|Default|GetElevatorPlayRate)) (/ (- 1.0 (Variables|Default|GetPreviousPlaybackPosition)) (LocalVariables|GetTotalTimeDifference)) 1e-06)
              (Development|PrintString (Utilities|String|Append (Utilities|String|ToString(Float) (/ 1.0 (Variables|Default|GetElevatorPlayRate))) " == " (Utilities|String|ToString(Float) (/ (- 1.0 (Variables|Default|GetPreviousPlaybackPosition)) (LocalVariables|GetTotalTimeDifference)))) true true "(R=0.109733,G=1.000000,B=0.000000,A=1.000000)" 1e+01)
              (else
                (Development|PrintString (Utilities|String|Append (Utilities|String|ToString(Float) (/ 1.0 (Variables|Default|GetElevatorPlayRate))) " =/= " (Utilities|String|ToString(Float) (/ (- 1.0 (Variables|Default|GetPreviousPlaybackPosition)) (LocalVariables|GetTotalTimeDifference)))) true true "(R=1.000000,G=0.000000,B=0.009181,A=1.000000)" 1e+01)))))))
    (:then_3
      (bind _output_get_4 (Variables|Default|SetElevatorPlayRate (/ (LocalVariables|GetNewTotalTimeDifference) (- 1.0 (Variables|Default|GetPreviousPlaybackPosition)))))
      (Components|Timeline|SetPlayRate (Variables|Default|GetElevatorMovement) (/ 1.0 _output_get_4))
      (Development|PrintString (Utilities|String|ToString(Float) _output_get_4) true true "(R=0.000000,G=0.660000,B=1.000000,A=1.000000)" 0.0)
      (return))))

(fn EndElevatorTime
  (params (TimeLeft :type Float%20%28single-precision%29))
  (CallFunction|UpdateElevatorTotalTime (+ TimeLeft (- (Utilities|Time|GetGameTimeinSeconds) (Variables|Default|GetElevatorStartTime)))))