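; BP_AbstractArtifact is a base Blueprint for artifacts that can glow and trigger a world transition.
; On BeginPlay it sets the glow component's emissive color from GetArtifactColor, a stub for child classes to supply, and zeroes the intensity.
; A timeline plays or reverses to fade the glow in and out, up to a small fixed maximum.
; World transition start and stop events forward to TransitionSphere when it is valid.
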(event EventBeginPlay
  (bind _bp_materialglowcomponent (Variables|Default|GetBP_MaterialGlowComponent))
  (|CallParentFunction)
  ;[1 1 1] Set the Default Emissive Glow
  (bind _emissivecolor (CallFunction|GetArtifactColor))
  (Default|SetEmissiveColor _bp_materialglowcomponent _emissivecolor)
  (Default|SetEmissiveIntensity _bp_materialglowcomponent 0.0)
  (Components|Timeline|SetPlayRate (Variables|Default|GetEmissiveTimeline) 1.0))

(event Collision|EventActorBeginOverlap
  (params (OtherActor :type Actor%20Object%20Reference)))

(event EventTick
  (params (DeltaSeconds :type Float%20%28single-precision%29)))

(event EventStartWorldTransition
  (bind _transitionsphere (Variables|Transition|GetTransitionSphere))
  (Utilities|IsValid _transitionsphere
    (:Is%20Valid
      (Default|StartWorldTransition _transitionsphere))))

(event EventStopWorldTransition
  (bind _transitionsphere (Variables|Transition|GetTransitionSphere))
  (Utilities|IsValid _transitionsphere
    (:Is%20Valid
      (Default|StopWorldTransition _transitionsphere))))

(event EventStartEmissiveGlow
  (bind _gradient (Timeline|EmissiveTimeline Play)
    (:Update
      (Default|SetEmissiveIntensity (Variables|Default|GetBP_MaterialGlowComponent) (* _gradient (Math|Float|MakeLiteralFloat 0.05))))))

(event EventStopEmissiveGlow
  (bind _gradient (Timeline|EmissiveTimeline Reverse)
    (:Update
      (Default|SetEmissiveIntensity (Variables|Default|GetBP_MaterialGlowComponent) (* _gradient (Math|Float|MakeLiteralFloat 0.05))))))

(fn ConstructionScript
  (|CallParentFunction))

(fn GetArtifactColor)