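; BP_GlobalFunctionLibrary is a Blueprint function library of shared helpers for a VR game.
; It fetches the VR game instance by cast, filters actor arrays by excluded class or required component, and toggles actor visibility through both hidden-in-game and propagated root-component visibility.
; EmergencyPrintMessage repeats on-screen prints so messages stand out, while PrintMessage has the same loop disconnected, so it prints nothing.
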(fn PrintMessage
  (params (Message :type String) (Duration :type Float%20%28single-precision%29) (Color :type Linear%20Color%20Structure)))

(fn GetVRGameInstance
  (params (WorldContext :type Object%20Object%20Reference))
  (bind _asmy_vrgame_instance_bp (Utilities|Casting|CastToMyVRGameInstanceBP (Game|GetGameInstance WorldContext))
    (:then
      (return _asmy_vrgame_instance_bp))
    (:CastFailed
      (return 0))))

(fn IgnoreFilterArray
  (params (TargetActors :type Array%20of%20Actor%20Object%20References) (ToIgnore :type Actor%20Class%20Reference))
  (for _array_element TargetActors
    (if (not (Utilities|ClassIsChildOf (Utilities|GetClass _array_element) ToIgnore))
      (Utilities|Array|Add (LocalVariables|GetLocalFilteredArray) _array_element)))
  (return (LocalVariables|GetLocalFilteredArray)))

(fn EmergencyPrintMessage
  (params (Message :type String) (Duration :type Float%20%28single-precision%29) (Color :type Linear%20Color%20Structure))
  ;[1 1 1] Print N times for Message to be Visible
  (for _index (range 0 20)
    (Development|PrintString 0 Message true false Color Duration)))

(fn SetTrueVisibility
  (params (Actors :type Array%20of%20Actor%20Object%20References) (IsVisible :type Boolean))
  (Rendering|SetActorHiddenInGame Actors (not IsVisible))
  (for _array_element Actors
    (Rendering|SetVisibility (VehicleSound|GetRootComponent _array_element) IsVisible true)))

(fn FilterActorsbyComponent
  (params (TargetActors :type Array%20of%20Actor%20Object%20References) (FilterBy :type Actor%20Component%20Class%20Reference))
  (for _array_element TargetActors
    (Utilities|IsValid (Actor|GetComponentbyClass _array_element FilterBy)
      (:Is%20Valid
        (Utilities|Array|Add (LocalVariables|GetLocalFilteredArray) _array_element))))
  (return (LocalVariables|GetLocalFilteredArray)))