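; BP_LabTable is an experimental lighting prop, apparently a lab table, with a configurable particle flame.
; The construction script passes Flame1 to SetFlameAttributes, which creates a dynamic material instance for its texture, flicker speed and emissive strength.
; The same function sets the particle's color, brightness and lifetime, randomizing flicker speed, brightness and lifetime within variable-defined ranges whenever construction runs.
; The event graph holds no active logic.
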(event EventBeginPlay)

(event Collision|EventActorBeginOverlap
  (params (OtherActor :type Actor%20Object%20Reference)))

(event EventTick
  (params (DeltaSeconds :type Float%20%28single-precision%29)))

(fn ConstructionScript
  (|CallParentFunction)
  (CallFunction|SetFlameAttributes (Variables|Default|GetFlame1)))

(fn SetFlameAttributes
  (params (FlameParticle :type Particle%20System%20Component%20Object%20Reference))
  (bind _returnvalue (Rendering|Material|CreateDynamicMaterialInstance FlameParticle 0 (Rendering|Material|GetMaterial FlameParticle 0) :!class /Script/Engine.PrimitiveComponent))
  (Rendering|Material|SetTextureParameterValue _returnvalue "FlameImage" (Variables|Default|GetFlameTexture))
  (Rendering|Material|SetScalarParameterValue _returnvalue "FlickerSpeed" (Math|Random|RandomFloatinRange (Variables|Default|GetFlameSway_Min) (Variables|Default|GetFlameSway_Max)) :!class /Script/Engine.MaterialInstanceDynamic)
  (Rendering|Material|SetScalarParameterValue _returnvalue "Emissive" (Variables|Default|GetFlameEmissiveStrength) :!class /Script/Engine.MaterialInstanceDynamic)
  (Effects|Components|ParticleSystem|SetColorParameter FlameParticle "Color" (Variables|Default|GetFlamecolor))
  (Effects|Components|ParticleSystem|SetFloatParameter FlameParticle "Brightness" (Math|Random|RandomFloatinRange (Variables|Default|GetBrightness_Min) (Variables|Default|GetBrightness_Max)))
  (Effects|Components|ParticleSystem|SetFloatParameter FlameParticle "Lifetime" (Math|Random|RandomFloatinRange (Variables|Default|GetFlicker_min) (Variables|Default|GetFlicker_max))))